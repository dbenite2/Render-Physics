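; BP_Constraint is a cable tether that physically links a sphere anchor to an object.
; On BeginPlay it constrains the referenced Object's mesh to the sphere and attaches the cable's end to it.
; When HaveEnd is false, a "Pickable" actor entering the box becomes the new constrained end, and the first-person character drops its held object.
; Breaking the constraint detaches the cable and clears HaveEnd.
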(event OnComponentBeginOverlap(Box)
  (params (OverlappedComponent :type Primitive%20Component%20Object%20Reference) (OtherActor :type Actor%20Object%20Reference) (OtherComp :type Primitive%20Component%20Object%20Reference) (OtherBodyIndex :type Integer) (bFromSweep :type Boolean) (SweepResult :type Hit%20Result%20Structure%20%28by%20ref%29))
  (if (not (Variables|Default|GetHaveEnd))
    (if (Actor|ActorHasTag OtherActor "Pickable")
      (bind _asbp_first_person_character (Utilities|Casting|CastToBP_FirstPersonCharacter (Game|Player|GetPlayerPawn 0)))
      (Class|PhysicsConstraintComponent|SetConstrainedComponents (Variables|Default|GetPhysicsConstraint) (Variables|Default|GetSphere) "None" OtherComp "None")
      (Class|CableComponent|SetAttachEndtoComponent (Variables|Default|GetCable) OtherComp "None")
      (Default|DropObject _asbp_first_person_character)
      (Variables|Default|SetHaveEnd true))))

(event OnConstraintBroken(PhysicsConstraint)
  (params (ConstraintIndex :type Integer))
  (Class|CableComponent|SetAttachEndtoComponent (Variables|Default|GetCable) 0 "None")
  (Variables|Default|SetHaveEnd false))

(event EventBeginPlay
  (bind _object (Variables|Default|GetObject))
  (bind _mesh (Variables|/Game/Blueprints/BP_PickableObject.BP_PickableObject_C|GetMesh _object))
  (Class|PhysicsConstraintComponent|SetConstrainedComponents (Variables|Default|GetPhysicsConstraint) (Variables|Default|GetSphere) "None" _mesh "None")
  (Class|CableComponent|SetAttachEndtoComponent (Variables|Default|GetCable) _mesh "None"))

(event Collision|EventActorBeginOverlap
  (params (OtherActor :type Actor%20Object%20Reference)))

(event EventTick
  (params (DeltaSeconds :type Float%20%28single-precision%29)))

(fn ConstructionScript)